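; Door is an actor that slides open when a player carrying the key enters its trigger box.
; The box overlap casts to BP_Player and checks HasKey, printing a hint to find the key when it is missing.
; With the key, a DoOnce stores the door's starting world location and plays a Timeline that offsets it along world Y, so it opens only once.
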(event `self.Box.OnComponentBeginOverlap`
  (params (OverlappedComponent :type "PrimitiveComponent Object Reference") (OtherActor :type "Actor Object Reference") (OtherComp :type "PrimitiveComponent Object Reference") (OtherBodyIndex :type Integer) (bFromSweep :type Boolean) (SweepResult :type "HitResult Structure (by ref)"))
  (bind (_initialdoorposition_x _initialdoorposition_y _initialdoorposition_z) (`KismetMathLibrary.BreakVector` (`self.InitialDoorPosition`)))
  (bind _asbp_player (cast `/Game/Blueprints/player/BP_Player` OtherActor))
  (if (`/Game/Blueprints/player/BP_Player.hasKey` _asbp_player)
    (`/Engine/EditorBlueprintResources/StandardMacros.DoOnce` false
      (:`Completed`
        (set `self.InitialDoorPosition` (`SceneComponent.K2_GetComponentLocation` (`self.Door`)))
        (bind (_direction _newtrack_0) (`Timeline|Timeline`)
          (:`Update`
            (`SceneComponent.K2_SetWorldLocation` (`self.Door`) (`KismetMathLibrary.MakeVector` _initialdoorposition_x (+ _newtrack_0 _initialdoorposition_y) _initialdoorposition_z) false false)))))
    (else
      (`KismetSystemLibrary.PrintString` "GO FIND THE KEY"))))

(event `self.Box.OnComponentEndOverlap`
  (params (OverlappedComponent :type "PrimitiveComponent Object Reference") (OtherActor :type "Actor Object Reference") (OtherComp :type "PrimitiveComponent Object Reference") (OtherBodyIndex :type Integer)))

(fn `UserConstructionScript`)